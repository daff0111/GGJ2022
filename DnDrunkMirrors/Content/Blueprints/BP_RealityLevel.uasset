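; Level actor that builds mirrored "realities" of the area inside RealityBox on each enabled Left, Right, Front or Back side.
; On BeginPlay it registers with the player's BP_MirroredCharacter and overlapping BP_MirroredObjectBase actors, spawning center actors and static mesh duplicates per side.
; Helpers mirror location, rotation and scale (negative Y) around centers offset by the box's full size, with GetMirroredTransform combining them for any actor.
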(event EventBeginPlay
  (bind _asbp_mirrored_character (Utilities|Casting|CastToBP_MirroredCharacter (Game|GetPlayerCharacter 0)))
  (bind _output_get (Variables|Default|SetMirrored%20Character _asbp_mirrored_character))
  (Default|SetupRealityLevel _output_get self)
  (Utilities|FlowControl|Delay 0.0)
  (Variables|Runtime|SetRealityStaticMeshes (Collision|GetOverlappingActors (Variables|Default|GetRealityBox) "/Script/Engine.StaticMeshActor" :!class /Script/Engine.PrimitiveComponent))
  (for _array_element (Variables|Realities|GetRealitySides)
    (CallFunction|SpawnReality _array_element)
    (CallFunction|CreateRealityMeshes _array_element))
  (bind _output_get_2 (Variables|Default|SetMirroredActors (Collision|GetOverlappingActors (Variables|Default|GetRealityBox) "/Game/Blueprints/MirroredObjects/BP_MirroredObjectBase.BP_MirroredObjectBase_C" :!class /Script/Engine.PrimitiveComponent)))
  (for _array_element_2 _output_get_2
    (bind _asbp_mirrored_object_base (Utilities|Casting|CastToBP_MirroredObjectBase _array_element_2))
    (Default|SetupRealiyLevel _asbp_mirrored_object_base self)))

(event Collision|EventActorBeginOverlap
  (params (OtherActor :type Actor%20Object%20Reference)))

(event EventTick
  (params (DeltaSeconds :type Float%20%28single-precision%29)))

(fn ConstructionScript)

(fn CreateRealityMeshes
  (params (RealitySide :type ERealitySide%20Enum :default "NewEnumerator0"))
  (bind _output_get (LocalVariables|SetCurrentRealitySide RealitySide))
  (switch Utilities|FlowControl|Switch|SwitchonERealitySide _output_get
    (:NewEnumerator0
      (if (Variables|Realities|GetLeftReality)
        (for _array_element (Variables|Runtime|GetRealityStaticMeshes) :!label _label
          (bind _asstatic_mesh_actor (Utilities|Casting|CastToStaticMeshActor _array_element))
          (LocalVariables|SetCurrentRelativeLocation (- (Transformation|GetWorldLocation (Variables|Default|GetRealityBox)) (Transformation|GetActorLocation _array_element)))
          (LocalVariables|SetCurrentScale (Transformation|GetActorScale3D _array_element))
          (LocalVariables|SetCurrentRelativeRotation (Transformation|GetActorRotation _array_element))
          (bind _returnvalue (Game|SpawnActorfromClass (Utilities|GetClass _array_element) (Math|Transform|MakeTransform (+ (Utilities|GetMirroredRelativeLocation (LocalVariables|GetCurrentRelativeLocation) (LocalVariables|GetCurrentRealitySide)) (Utilities|GetRealityCenter (LocalVariables|GetCurrentRealitySide))) (Utilities|GetMirroredRelativeRotation (LocalVariables|GetCurrentRelativeRotation) (LocalVariables|GetCurrentRealitySide)) (Utilities|GetMirroredRelativeScale (LocalVariables|GetCurrentScale) (LocalVariables|GetCurrentRealitySide))) "AlwaysSpawn" _asstatic_mesh_actor 0))
          (bind _asstatic_mesh_actor_2 (Utilities|Casting|CastToStaticMeshActor _returnvalue))
          (Transformation|SetMobility _asstatic_mesh_actor_2 "Movable")
          (Rendering|SetVisibility (Variables|/Script/Engine.StaticMeshActor|GetStaticMeshComponent _asstatic_mesh_actor_2) (Variables|/Script/Engine.SceneComponent|GetbVisible (Variables|/Script/Engine.StaticMeshActor|GetStaticMeshComponent _asstatic_mesh_actor)) false)
          (Collision|SetCollisionEnabled (Variables|/Script/Engine.StaticMeshActor|GetStaticMeshComponent _asstatic_mesh_actor_2) (Collision|GetCollisionEnabled (Variables|/Script/Engine.StaticMeshActor|GetStaticMeshComponent _asstatic_mesh_actor)))
          (Components|StaticMesh|SetStaticMesh (Variables|/Script/Engine.StaticMeshActor|GetStaticMeshComponent _asstatic_mesh_actor_2) (Variables|/Script/Engine.StaticMeshComponent|GetStaticMesh (Variables|/Script/Engine.StaticMeshActor|GetStaticMeshComponent _asstatic_mesh_actor)))
          (for (_array_element_2 _array_index) (Rendering|Material|GetMaterials (Variables|/Script/Engine.StaticMeshActor|GetStaticMeshComponent _asstatic_mesh_actor))
            (Rendering|Material|SetMaterial (Variables|/Script/Engine.StaticMeshActor|GetStaticMeshComponent _asstatic_mesh_actor_2) _array_index _array_element_2))
          (Transformation|SetMobility _asstatic_mesh_actor_2 "Static"))))
    (:NewEnumerator1
      (if (Variables|Realities|GetRightReality)
        (goto _label)))
    (:NewEnumerator2
      (if (Variables|Realities|GetFrontReality)
        (goto _label)))
    (:NewEnumerator3
      (if (Variables|Realities|GetBackReality)
        (goto _label)))))

(fn SpawnReality
  (params (RealitySide :type ERealitySide%20Enum :default "NewEnumerator0"))
  (bind _output_get (LocalVariables|SetCurrentRealitySide RealitySide))
  (switch Utilities|FlowControl|Switch|SwitchonERealitySide _output_get
    (:NewEnumerator0
      (if (Variables|Realities|GetLeftReality)
        (bind _returnvalue (Game|SpawnActorfromClass "/Script/Engine.Actor" (Math|Transform|MakeTransform (Utilities|GetRealityCenter _output_get) "0, 0, 0" "1,1,1") "Undefined" 0 0 :!label _label))
        (Utilities|Array|Add (Variables|Realities|GetRealitiesCenters) _returnvalue)))
    (:NewEnumerator1
      (if (Variables|Realities|GetRightReality)
        (goto _label)))
    (:NewEnumerator2
      (if (Variables|Realities|GetFrontReality)
        (goto _label)))
    (:NewEnumerator3
      (if (Variables|Realities|GetBackReality)
        (goto _label)))))

(fn GetMirroredTransform
  (params (Actor :type Actor%20Object%20Reference) (RealitySide :type ERealitySide%20Enum :default "NewEnumerator0"))
  (bind _returnvalue (Transformation|GetActorTransform Actor))
  (return (Math|Transform|MakeTransform (+ (Utilities|GetRealityCenter RealitySide) (Utilities|GetMirroredRelativeLocation (- (Transformation|GetWorldLocation (Variables|Default|GetRealityBox)) (.location _returnvalue)) RealitySide)) (Utilities|GetMirroredRelativeRotation (.rotation _returnvalue) RealitySide) (Utilities|GetMirroredRelativeScale (.scale _returnvalue) RealitySide))))