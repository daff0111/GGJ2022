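; BP_Door is an interactable, lockable swinging door among the mirrored objects that toggles open and closed on interaction.
; Timelines drive its yaw relative to the starting rotation, with sound cues, and release the interactable component when finished.
; Opening also hides an optional Wall mesh.
; Locking works by marking the component as already being interacted with; an auto-toggle loop keyed on MirroredSide is left disconnected.
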(event StartInteracting(BP_InteractableComponent)
  (if (Variables|Default|GetIsOpen)
    (CallFunction|CloseDoor)
    (else
      (CallFunction|OpenDoor))))

(event Custom|Close%20Door
  (bind _returnvalue (Transformation|GetActorRotation))
  (Audio|PlaySoundatLocation "/Game/Audio/open-door_Cue.open-door_Cue" (Transformation|GetActorLocation) "0, 0, 0" 1.0 1.0 0.0 0 0 0)
  (bind _rotation (Timeline|CloseTimelie PlayFromStart)
    (:Update
      (Transformation|SetActorRotation (Math|Rotator|MakeRotator (.roll _returnvalue) (.pitch _returnvalue) (+ (Variables|Default|GetStartRotation) _rotation))))
    (:Finished
      (Default|Interact (Variables|Default|GetBP_InteractableComponent) false)
      (Variables|Default|SetIsOpen false)
      (Audio|PlaySoundatLocation "/Game/Audio/door-close_Cue.door-close_Cue" (Transformation|GetActorLocation) "0, 0, 0" 1.0 1.0 0.0 0 0 0))))

(event Custom|LockDoor
  (params (IsLocked :type Boolean))
  (bind _output_get (Variables|Mirror|SetIsLocked IsLocked))
  (Variables|/Game/Blueprints/MirroredObjects/InteractableObjects/BP_InteractableComponent.BP_InteractableComponent_C|SetIsBeingInteracted (Variables|Default|GetBP_InteractableComponent) _output_get))

(event Custom|Open%20Door
  (bind _returnvalue (Transformation|GetActorRotation))
  (bind _wall (Variables|Default|GetWall))
  (Utilities|IsValid _wall
    (:Is%20Valid
      (Rendering|SetVisibility (Variables|/Script/Engine.StaticMeshActor|GetStaticMeshComponent _wall) false false))
    (:Is%20Not%20Valid
      _))
  (Audio|PlaySoundatLocation "/Game/Audio/open-door_Cue.open-door_Cue" (Transformation|GetActorLocation) "0, 0, 0" 1.0 1.0 0.0 0 0 0)
  (bind _rotation (Timeline|OpenTimeline PlayFromStart)
    (:Update
      (Transformation|SetActorRotation (Math|Rotator|MakeRotator (.roll _returnvalue) (.pitch _returnvalue) (+ (Variables|Default|GetStartRotation) _rotation))))
    (:Finished
      (Default|Interact (Variables|Default|GetBP_InteractableComponent) false)
      (Variables|Default|SetIsOpen true))))

(event EventBeginPlay
  (|CallParentFunction)
  (Variables|Default|SetStartRotation (.yaw (Transformation|GetActorRotation)))
  (Variables|/Game/Blueprints/MirroredObjects/InteractableObjects/BP_InteractableComponent.BP_InteractableComponent_C|SetIsBeingInteracted (Variables|Default|GetBP_InteractableComponent) (Variables|Mirror|GetIsLocked)))

(fn ConstructionScript
  (|CallParentFunction))