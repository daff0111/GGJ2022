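; Component that makes an object interactable and highlightable, tracking whether it is being interacted with or highlighted.
; Interact and Highlight store the new state and call matching dispatchers for start/stop interacting and highlight on/off, leaving the actual response to listeners.
; CanInteract allows interaction only while the object is not already being interacted with.
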(event EventBeginPlay)

(event EventTick
  (params (DeltaSeconds :type Float%20%28single-precision%29)))

(fn Interact
  (params (IsBeingInteracted :type Boolean))
  (bind _output_get (Variables|Default|SetIsBeingInteracted IsBeingInteracted))
  (if _output_get
    (Default|CallStartInteracting)
    (else
      (Default|CallStopInteracting))))

(fn CanInteract
  (return (not (Variables|Default|GetIsBeingInteracted))))

(fn Highlight
  (params (IsHighlighted :type Boolean))
  (bind _output_get (Variables|Default|SetIsHighlighted IsHighlighted))
  (if _output_get
    (Default|CallHighlighton)
    (else
      (Default|CallHighlightOff))))