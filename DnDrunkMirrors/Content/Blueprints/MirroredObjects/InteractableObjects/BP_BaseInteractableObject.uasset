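; Base Blueprint for interactable mirrored objects that show a highlight across reality and its mirror copies.
; Interactable component highlight events are handled only on the Real-side instance.
; It loops the level's reality sides, toggling the highlight mesh on the Left, Right, Front and Back copies and itself wherever RealityVisibility allows.
; Reality level setup extends the parent and starts the highlight hidden.
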(event Highlighton(BP_InteractableComponent)
  (if (Utilities|Enum|Equal(Enum) (Variables|Default|GetMirroredSide) "NewEnumerator4")
    (for _array_element (Variables|/Game/Blueprints/BP_RealityLevel.BP_RealityLevel_C|GetRealitySides (Variables|Default|GetRealityLevel))
      (if (.Value (Utilities|Map|Find (Variables|Default|GetRealityVisibility) _array_element))
        (bind _asbp_base_interactable_object (Utilities|Casting|CastToBP_BaseInteractableObject (Utilities|Select :Index _array_element :NewEnumerator0 (Variables|Default|GetLeftMirrorObject) :NewEnumerator1 (Variables|Default|GetRightMirrorObject) :NewEnumerator2 (Variables|Default|GetFrontMirrorObject) :NewEnumerator3 (Variables|Default|GetBackMirrorObject) :NewEnumerator4 0)))
        (CallFunction|SetHighlight _asbp_base_interactable_object true)))
    (if (.Value (Utilities|Map|Find (Variables|Default|GetRealityVisibility) "NewEnumerator4"))
      (CallFunction|SetHighlight true))))

(event HighlightOff(BP_InteractableComponent)
  (if (Utilities|Enum|Equal(Enum) (Variables|Default|GetMirroredSide) "NewEnumerator4")
    (for _array_element (Variables|/Game/Blueprints/BP_RealityLevel.BP_RealityLevel_C|GetRealitySides (Variables|Default|GetRealityLevel))
      (if (.Value (Utilities|Map|Find (Variables|Default|GetRealityVisibility) _array_element))
        (bind _asbp_base_interactable_object (Utilities|Casting|CastToBP_BaseInteractableObject (Utilities|Select :Index _array_element :NewEnumerator0 (Variables|Default|GetLeftMirrorObject) :NewEnumerator1 (Variables|Default|GetRightMirrorObject) :NewEnumerator2 (Variables|Default|GetFrontMirrorObject) :NewEnumerator3 (Variables|Default|GetBackMirrorObject) :NewEnumerator4 self)))
        (CallFunction|SetHighlight _asbp_base_interactable_object false)))
    (if (.Value (Utilities|Map|Find (Variables|Default|GetRealityVisibility) "NewEnumerator4"))
      (CallFunction|SetHighlight false))))

(event Custom|SetHighlight
  (params (bNewVisibility :type Boolean))
  (Rendering|SetVisibility (Variables|Default|GetStaticMeshHighlight) bNewVisibility true))

(event EventBeginPlay
  (|CallParentFunction) ; This node is disabled and will not be called.\nDrag off pins to build functionality.
)

(event Collision|EventActorBeginOverlap
  (params (OtherActor :type Actor%20Object%20Reference))
  (|CallParentFunction OtherActor) ; This node is disabled and will not be called.\nDrag off pins to build functionality.
)

(event EventTick
  (params (DeltaSeconds :type Float%20%28single-precision%29))
  (|CallParentFunction DeltaSeconds) ; This node is disabled and will not be called.\nDrag off pins to build functionality.
)

(fn ConstructionScript
  (|CallParentFunction))

(fn SetupRealiyLevel
  (params (RealityLevel :type BP%20Reality%20Level%20Object%20Reference))
  (|CallParentFunction RealityLevel)
  (Rendering|SetVisibility (Variables|Default|GetStaticMeshHighlight) false false))