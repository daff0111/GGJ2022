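; Base Blueprint for pickupable objects that have mirrored counterparts across reality sides, driven by BP_InteractableComponent events.
; Starting interaction flags the object as picked up, disables physics, snaps the mesh to its root and switches collision to query-only overlap.
; It also re-snaps mirror copies' meshes for each side in RealityLevel.RealitySides.
; Stopping restores physics and blocking collision on its own mesh only; ThrowObject is an empty event.
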(event StartInteracting(BP_InteractableComponent)
  (bind _staticmesh (Variables|Default|GetStaticMesh))
  (CallFunction|PickupObject true)
  (Physics|SetSimulatePhysics _staticmesh false)
  (Transformation|AttachComponentToComponent (Variables|Default|GetStaticMesh) (Variables|Default|GetDefaultSceneRoot) "None" "SnapToTarget" "SnapToTarget" "KeepWorld" true)
  (Collision|SetCollisionResponsetoAllChannels _staticmesh "ECR_Overlap")
  (Collision|SetCollisionEnabled _staticmesh "QueryOnly")
  (for _array_element (Variables|/Game/Blueprints/BP_RealityLevel.BP_RealityLevel_C|GetRealitySides (Variables|Default|GetRealityLevel))
    (bind _asbp_base_pickupable_object (Utilities|Casting|CastToBP_BasePickupableObject (Utilities|Select :Index _array_element :NewEnumerator0 (Variables|Default|GetLeftMirrorObject) :NewEnumerator1 (Variables|Default|GetRightMirrorObject) :NewEnumerator2 (Variables|Default|GetFrontMirrorObject) :NewEnumerator3 (Variables|Default|GetBackMirrorObject) :NewEnumerator4 0)))
    (Transformation|AttachComponentToComponent (Variables|/Game/Blueprints/MirroredObjects/BP_StaticMesh_MirroredObject.BP_StaticMesh_MirroredObject_C|GetStaticMesh _asbp_base_pickupable_object) (Variables|/Game/Blueprints/MirroredObjects/BP_MirroredObjectBase.BP_MirroredObjectBase_C|GetDefaultSceneRoot _asbp_base_pickupable_object) "None" "SnapToTarget" "SnapToTarget" "KeepWorld" true)))

(event StopInteracting(BP_InteractableComponent)
  (bind _staticmesh (Variables|Default|GetStaticMesh))
  (CallFunction|PickupObject false)
  (Physics|SetSimulatePhysics _staticmesh true)
  (Collision|SetCollisionResponsetoAllChannels _staticmesh "ECR_Block")
  (Collision|SetCollisionEnabled _staticmesh "QueryAndPhysics"))

(event Custom|ThrowObject)

(event Custom|PickupObject
  (params (IsPickedUp :type Boolean))
  (Variables|Default|SetIsPickedUp IsPickedUp))

(event EventBeginPlay
  (|CallParentFunction) ; This node is disabled and will not be called.\nDrag off pins to build functionality.
)

(event Collision|EventActorBeginOverlap
  (params (OtherActor :type Actor%20Object%20Reference))
  (|CallParentFunction OtherActor) ; This node is disabled and will not be called.\nDrag off pins to build functionality.
)

(event EventTick
  (params (DeltaSeconds :type Float%20%28single-precision%29))
  (|CallParentFunction DeltaSeconds) ; This node is disabled and will not be called.\nDrag off pins to build functionality.
)

(fn ConstructionScript
  (|CallParentFunction))