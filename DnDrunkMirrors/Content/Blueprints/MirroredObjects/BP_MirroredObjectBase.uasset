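; Base actor for objects that appear mirrored in the side realities of a reality level.
; SetupRealiyLevel stores the level and spawns a same-class copy for each enabled Left, Right, Front or Back side, tagging it with its side via SetupCopy.
; Tick calls UpdateCopies, which moves each valid copy to the location and rotation from the level's GetMirroredTransform.
; Copies never receive the level here, so only the original drives updates.
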(event EventBeginPlay)

(event Collision|EventActorBeginOverlap
  (params (OtherActor :type Actor%20Object%20Reference)))

(event EventTick
  (params (DeltaSeconds :type Float%20%28single-precision%29))
  (CallFunction|UpdateCopies DeltaSeconds))

(fn ConstructionScript)

(fn CreateCopy
  (params (RealitySide :type ERealitySide%20Enum :default "NewEnumerator0") (Object :type BP%20Mirrored%20Object%20Base%20Object%20Reference) (SpawnTransform :type Transform))
  (bind _returnvalue (Game|SpawnActorfromClass (Utilities|GetClass Object) SpawnTransform "Undefined" 0 0))
  (switch Utilities|FlowControl|Switch|SwitchonERealitySide RealitySide
    (:NewEnumerator0
      (Variables|Default|SetLeftMirrorObject _returnvalue))
    (:NewEnumerator1
      (Variables|Default|SetRightMirrorObject _returnvalue))
    (:NewEnumerator2
      (Variables|Default|SetFrontMirrorObject _returnvalue))
    (:NewEnumerator3
      (Variables|Default|SetBackMirrorObject _returnvalue)))
  (return _returnvalue))

(fn SetupCopy
  (params (MirroredSide :type ERealitySide%20Enum :default "NewEnumerator0") (BaseObject :type BP%20Mirrored%20Object%20Base%20Object%20Reference))
  (Variables|Default|SetMirroredSide MirroredSide))

(fn SetupRealiyLevel
  (params (RealityLevel :type BP%20Reality%20Level%20Object%20Reference))
  (bind _output_get (Variables|Default|SetRealityLevel RealityLevel))
  (for _array_element (Variables|/Game/Blueprints/BP_RealityLevel.BP_RealityLevel_C|GetRealitySides _output_get)
    (switch Utilities|FlowControl|Switch|SwitchonERealitySide _array_element
      (:NewEnumerator0
        (if (Variables|/Game/Blueprints/BP_RealityLevel.BP_RealityLevel_C|GetLeftReality (Variables|Default|GetRealityLevel))
          (bind _newobject (CallFunction|CreateCopy _array_element self (Default|GetMirroredTransform (Variables|Default|GetRealityLevel) self _array_element) :!label _label))
          (CallFunction|SetupCopy _newobject _array_element self)))
      (:NewEnumerator1
        (if (Variables|/Game/Blueprints/BP_RealityLevel.BP_RealityLevel_C|GetRightReality (Variables|Default|GetRealityLevel))
          (goto _label)))
      (:NewEnumerator2
        (if (Variables|/Game/Blueprints/BP_RealityLevel.BP_RealityLevel_C|GetFrontReality (Variables|Default|GetRealityLevel))
          (goto _label)))
      (:NewEnumerator3
        (if (Variables|/Game/Blueprints/BP_RealityLevel.BP_RealityLevel_C|GetBackReality (Variables|Default|GetRealityLevel))
          (goto _label))))))

(fn UpdateCopies
  (params (DeltaSeconds :type Float%20%28single-precision%29))
  (bind _realitylevel (Variables|Default|GetRealityLevel))
  (Utilities|IsValid _realitylevel
    (:Is%20Valid
      (for _array_element (Variables|/Game/Blueprints/BP_RealityLevel.BP_RealityLevel_C|GetRealitySides _realitylevel)
        (Utilities|IsValid (Utilities|Select :Index _array_element :NewEnumerator0 (Variables|Default|GetLeftMirrorObject) :NewEnumerator1 (Variables|Default|GetRightMirrorObject) :NewEnumerator2 (Variables|Default|GetFrontMirrorObject) :NewEnumerator3 (Variables|Default|GetBackMirrorObject) :NewEnumerator4 0)
          (:Is%20Valid
            (Transformation|SetActorLocationAndRotation (Utilities|Select :Index _array_element :NewEnumerator0 (Variables|Default|GetLeftMirrorObject) :NewEnumerator1 (Variables|Default|GetRightMirrorObject) :NewEnumerator2 (Variables|Default|GetFrontMirrorObject) :NewEnumerator3 (Variables|Default|GetBackMirrorObject) :NewEnumerator4 0) (.location (Default|GetMirroredTransform (Variables|Default|GetRealityLevel) self _array_element)) (.rotation (Default|GetMirroredTransform (Variables|Default|GetRealityLevel) self _array_element)))))))))