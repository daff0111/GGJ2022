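; BP_Button is a mirrored pressure plate that reveals a linked door and makes it interactable while pressed.
; At BeginPlay it hides and locks the door after a short delay.
; On the Real side, mirrored characters or balls entering its sphere press it; exits release it only when no balls remain.
; PressButton toggles the door, plays a click and rescales the plate and its mirror copies across the level's reality sides.
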(event OnComponentBeginOverlap(Sphere)
  (params (OverlappedComponent :type Primitive%20Component%20Object%20Reference) (OtherActor :type Actor%20Object%20Reference) (OtherComp :type Primitive%20Component%20Object%20Reference) (OtherBodyIndex :type Integer) (bFromSweep :type Boolean) (SweepResult :type Hit%20Result%20Structure%20%28by%20ref%29))
  (if (Utilities|Enum|Equal(Enum) (Variables|Default|GetMirroredSide) "NewEnumerator4")
    (Utilities|Casting|CastToBP_MirroredCharacter OtherActor
      (:then
        _)
      (:CastFailed
        (Utilities|Casting|CastToBP_MirroredBall OtherActor)))
    (if (not (Variables|Default|GetIsPressed))
      (CallFunction|PressButton true))))

(event OnComponentEndOverlap(Sphere)
  (params (OverlappedComponent :type Primitive%20Component%20Object%20Reference) (OtherActor :type Actor%20Object%20Reference) (OtherComp :type Primitive%20Component%20Object%20Reference) (OtherBodyIndex :type Integer))
  (if (Utilities|Enum|Equal(Enum) (Variables|Default|GetMirroredSide) "NewEnumerator4")
    (Utilities|Casting|CastToBP_MirroredCharacter OtherActor
      (:then
        _)
      (:CastFailed
        (Utilities|Casting|CastToBP_MirroredBall OtherActor)))
    (if (and (< (Utilities|Array|Length (Collision|GetOverlappingActors (Variables|Default|GetSphere) "/Game/Blueprints/MirroredObjects/BP_MirroredBall.BP_MirroredBall_C" :!class /Script/Engine.PrimitiveComponent)) 1) (Variables|Default|GetIsPressed))
      (CallFunction|PressButton false))))

(event Custom|PressButton
  (params (IsPressed :type Boolean))
  (bind _door (Variables|Default|GetDoor))
  (bind _realitylevel (Variables|Default|GetRealityLevel))
  (Utilities|IsValid _realitylevel
    (:Is%20Valid
      (bind _output_get (Variables|Default|SetIsPressed IsPressed))
      (Utilities|FlowControl|Sequence
        (:then_0
          (Audio|PlaySoundatLocation (select _output_get "/Game/Audio/click26_Cue.click26_Cue" "/Game/Audio/unclick_Cue.unclick_Cue") (Transformation|GetActorLocation) "0, 0, 0" 1.0 1.0 0.0 0 0 0)
          (Utilities|IsValid _door
            (:Is%20Valid
              (Rendering|SetVisibility (Variables|/Game/Blueprints/MirroredObjects/BP_StaticMesh_MirroredObject.BP_StaticMesh_MirroredObject_C|GetStaticMesh _door) _output_get false)
              (Utilities|Map|Add (Variables|/Game/Blueprints/MirroredObjects/BP_StaticMesh_MirroredObject.BP_StaticMesh_MirroredObject_C|GetRealityVisibility _door) "NewEnumerator4" _output_get)
              (Variables|/Game/Blueprints/MirroredObjects/InteractableObjects/BP_InteractableComponent.BP_InteractableComponent_C|SetIsBeingInteracted (Variables|/Game/Blueprints/MirroredObjects/InteractableObjects/BP_BaseInteractableObject.BP_BaseInteractableObject_C|GetBP_InteractableComponent _door) (not _output_get))
              (if _output_get
                (Default|SetHighlight _door false)))))
        (:then_1
          (Transformation|SetWorldScale3D (Variables|Default|GetStaticMesh) (select _output_get "0.800000,0.800000,0.100000" "0.800000,0.800000,0.200000"))
          (for _array_element (Variables|/Game/Blueprints/BP_RealityLevel.BP_RealityLevel_C|GetRealitySides _realitylevel)
            (bind _asbp_static_mesh_mirrored_object (Utilities|Casting|CastToBP_StaticMesh_MirroredObject (Utilities|Select :Index _array_element :NewEnumerator0 (Variables|Default|GetLeftMirrorObject) :NewEnumerator1 (Variables|Default|GetRightMirrorObject) :NewEnumerator2 (Variables|Default|GetFrontMirrorObject) :NewEnumerator3 (Variables|Default|GetBackMirrorObject) :NewEnumerator4 0)))
            (Transformation|SetWorldScale3D (Variables|/Game/Blueprints/MirroredObjects/BP_StaticMesh_MirroredObject.BP_StaticMesh_MirroredObject_C|GetStaticMesh _asbp_static_mesh_mirrored_object) (select _output_get "0.800000,-0.800000,0.100000" "0.800000,-0.800000,0.200000"))))))))

(event EventBeginPlay
  (bind _door (Variables|Default|GetDoor))
  (|CallParentFunction)
  (Utilities|FlowControl|Delay 0.2)
  (Utilities|IsValid _door
    (:Is%20Valid
      (Rendering|SetVisibility (Variables|/Game/Blueprints/MirroredObjects/BP_StaticMesh_MirroredObject.BP_StaticMesh_MirroredObject_C|GetStaticMesh _door) false false)
      (Utilities|Map|Add (Variables|/Game/Blueprints/MirroredObjects/BP_StaticMesh_MirroredObject.BP_StaticMesh_MirroredObject_C|GetRealityVisibility _door) "NewEnumerator4" false)
      (if true
        (Default|SetHighlight _door false)
        (Variables|/Game/Blueprints/MirroredObjects/InteractableObjects/BP_InteractableComponent.BP_InteractableComponent_C|SetIsBeingInteracted (Variables|/Game/Blueprints/MirroredObjects/InteractableObjects/BP_BaseInteractableObject.BP_BaseInteractableObject_C|GetBP_InteractableComponent _door) true)))))

(event EventTick
  (params (DeltaSeconds :type Float%20%28single-precision%29))
  (|CallParentFunction DeltaSeconds) ; This node is disabled and will not be called.\nDrag off pins to build functionality.
)

(fn ConstructionScript
  (|CallParentFunction))