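; A collectible pickup that exists in reality with mirror copies on other sides of the level.
; A looping timeline continuously spins its yaw.
; When a BP_MirroredCharacter overlaps the sphere of the Real-side instance, it fires once, playing a pickup sound at its location.
; It then destroys its valid Left, Right, Front and Back mirror objects, selected through the level's RealitySides, and finally itself.
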(event OnComponentBeginOverlap(Sphere)
  (params (OverlappedComponent :type Primitive%20Component%20Object%20Reference) (OtherActor :type Actor%20Object%20Reference) (OtherComp :type Primitive%20Component%20Object%20Reference) (OtherBodyIndex :type Integer) (bFromSweep :type Boolean) (SweepResult :type Hit%20Result%20Structure%20%28by%20ref%29))
  (Utilities|Casting|CastToBP_MirroredCharacter OtherActor)
  (if (Utilities|Enum|Equal(Enum) (Variables|Default|GetMirroredSide) "NewEnumerator4")
    (Utilities|FlowControl|DoOnce false
      (:Completed
        (CallFunction|Collect)
        (CallFunction|Destroy)))))

(event EventBeginPlay
  (|CallParentFunction)
  (bind _newtrack_0 (Timeline|RotationLoop Play)
    (:Update
      (Transformation|SetActorRotation (Math|Rotator|MakeRotator 0.0 0.0 _newtrack_0)))
    (:Finished
      (Utilities|FlowControl|Delay 0.0)
      (Timeline|RotationLoop PlayFromStart))))

(event Collision|EventActorBeginOverlap
  (params (OtherActor :type Actor%20Object%20Reference))
  (|CallParentFunction OtherActor) ; This node is disabled and will not be called.\nDrag off pins to build functionality.
)

(event EventTick
  (params (DeltaSeconds :type Float%20%28single-precision%29))
  (|CallParentFunction DeltaSeconds) ; This node is disabled and will not be called.\nDrag off pins to build functionality.
)

(fn ConstructionScript
  (|CallParentFunction))

(fn Collect
  (Audio|PlaySoundatLocation (Variables|Default|GetSound) (Transformation|GetActorLocation) "0, 0, 0" 1.0 1.0 0.0 0 0 0))

(fn Destroy
  (for _array_element (Variables|/Game/Blueprints/BP_RealityLevel.BP_RealityLevel_C|GetRealitySides (Variables|Default|GetRealityLevel))
    (Utilities|IsValid (Utilities|Select :Index _array_element :NewEnumerator0 (Variables|Default|GetLeftMirrorObject) :NewEnumerator1 (Variables|Default|GetRightMirrorObject) :NewEnumerator2 (Variables|Default|GetFrontMirrorObject) :NewEnumerator3 (Variables|Default|GetBackMirrorObject) :NewEnumerator4 0)
      (:Is%20Valid
        (Actor|DestroyActor (Utilities|Select :Index _array_element :NewEnumerator0 (Variables|Default|GetLeftMirrorObject) :NewEnumerator1 (Variables|Default|GetRightMirrorObject) :NewEnumerator2 (Variables|Default|GetFrontMirrorObject) :NewEnumerator3 (Variables|Default|GetBackMirrorObject) :NewEnumerator4 0)))))
  (Actor|DestroyActor))