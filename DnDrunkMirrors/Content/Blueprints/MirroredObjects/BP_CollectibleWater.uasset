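; BP_CollectibleWater is a water pickup that changes the player's drunk level when collected.
; On BeginPlay it finds the level's BP_DrunkManager with GetActorOfClass and caches the reference.
; Its Collect override runs the parent's collect logic, then passes its DrunkLevel value to the manager's AddDrunkLevel.
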(event EventBeginPlay
  (|CallParentFunction)
  (bind _returnvalue (Actor|GetActorOfClass "/Game/Blueprints/BP_DrunkManager.BP_DrunkManager_C"))
  (Variables|Default|SetDrunkManager _returnvalue))

(event Collision|EventActorBeginOverlap
  (params (OtherActor :type Actor%20Object%20Reference))
  (|CallParentFunction OtherActor) ; This node is disabled and will not be called.\nDrag off pins to build functionality.
)

(event EventTick
  (params (DeltaSeconds :type Float%20%28single-precision%29))
  (|CallParentFunction DeltaSeconds) ; This node is disabled and will not be called.\nDrag off pins to build functionality.
)

(fn ConstructionScript
  (|CallParentFunction))

(fn Collect
  (|CallParentFunction)
  (Default|AddDrunkLevel (Variables|Default|GetDrunkManager) (Variables|Default|GetDrunkLevel)))