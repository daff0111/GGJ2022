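; Manager Blueprint that holds the drunkenness level and drives the Amount scalar in the MPC_Drunk material parameter collection.
; SetDrunkLevel and AddDrunkLevel keep the level clamped between zero and one; BeginPlay starts it at maximum.
; A timeline, restarted through a zero-length delay whenever it finishes, continually varies Amount between a slightly reduced level and the current one.
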(event Custom|SetDrunkLevel
  (params (DrunkFloat :type Float%20%28single-precision%29))
  (Variables|Default|SetDrunkFloat (Math|Float|Clamp(Float) DrunkFloat)))

(event Custom|Add%20Drunk%20Level
  (params (Level :type Float%20%28single-precision%29))
  (CallFunction|SetDrunkLevel (+ Level (Variables|Default|GetDrunkFloat))))

(event EventBeginPlay
  (bind _drunkfloat (Variables|Default|GetDrunkFloat))
  (CallFunction|SetDrunkLevel 1.0)
  (bind _alpha (Timeline|Timeline_0 Play)
    (:Update
      (Rendering|Material|SetScalarParameterValue "/Game/Materials/MPC_Drunk.MPC_Drunk" "Amount" (Math|Float|Lerp (Math|Float|Clamp(Float) (- _drunkfloat 0.2) 0.01 1.0) _drunkfloat _alpha) :!class /Script/Engine.KismetMaterialLibrary))
    (:Finished
      (Utilities|FlowControl|Delay 0.0)
      (Timeline|Timeline_0 PlayFromStart))))

(event Collision|EventActorBeginOverlap
  (params (OtherActor :type Actor%20Object%20Reference)))

(event EventTick
  (params (DeltaSeconds :type Float%20%28single-precision%29)))

(fn ConstructionScript)